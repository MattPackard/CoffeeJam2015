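; Boulder trap for a side-scroller that launches a physics boulder when the player character overlaps its trigger box.
; The trigger fires once, playing a sound, enabling simulation and applying a velocity-change impulse along the Impulse component's forward vector, scaled by StartingForce.
; Boulder hits call HandleDeath on the character while CanKillP is true, which a fixed delay after launch clears.
; An unconnected velocity check targeting a separate KillPlayer flag never runs.
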(event OnComponentBeginOverlap(Box)
  (params (OtherActor :type Actor%20Object%20Reference) (OtherComp :type Primitive%20Component%20Object%20Reference) (OtherBodyIndex :type Integer) (bFromSweep :type Boolean) (SweepResult :type Hit%20Result%20Structure%20%28by%20ref%29))
  (bind _boulder (Variables|Default|GetBoulder))
  (Utilities|Casting|CastToSideScrollerCharacter OtherActor)
  (Utilities|FlowControl|DoOnce false
    (:Completed
      (Audio|PlaySound2D "/Game/Sounds/SFX/traps/BoulderCue.BoulderCue" 1.0 1.0)
      (Physics|SetSimulatePhysics _boulder true)
      (Physics|AddImpulse _boulder (* (Math|Vector|GetForwardVector (Variables|Default|GetImpulse)) (Variables|Default|GetStarting%20Force)) "None" true)
      (Utilities|FlowControl|Delay 2.4)
      (Variables|Default|SetcanKillP false))))

(event OnComponentHit(Boulder)
  (params (OtherActor :type Actor%20Object%20Reference) (OtherComp :type Primitive%20Component%20Object%20Reference) (NormalImpulse :type Vector :default "0, 0, 0") (Hit :type Hit%20Result%20Structure%20%28by%20ref%29))
  (bind _asside_scroller_character (Utilities|Casting|CastToSideScrollerCharacter OtherActor))
  (if (Variables|Default|GetcanKillP)
    (Default|HandleDeath _asside_scroller_character)))

(event EventTick
  (params (DeltaSeconds :type Float%20%28single-precision%29)))

(fn ConstructionScript)
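; BP_FlameThrower is a trap that cycles a flame on and off and kills any SideScrollerCharacter that begins overlapping its kill zone while lit.
; After a configurable start delay, StartFire and StopFire schedule each other through one-shot timers using separate fire and idle durations.
; Each switch toggles the flame's visibility, the KillZone's query collision and a spawned looping-or-stopped flamethrower sound.
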(event OnComponentBeginOverlap(KillZone)
  (params (OtherActor :type Actor%20Object%20Reference) (OtherComp :type Primitive%20Component%20Object%20Reference) (OtherBodyIndex :type Integer) (bFromSweep :type Boolean) (SweepResult :type Hit%20Result%20Structure%20%28by%20ref%29))
  (bind _asside_scroller_character (Utilities|Casting|CastToSideScrollerCharacter OtherActor))
  (Default|CallOnDeath _asside_scroller_character))

(event Custom|StopFire
  (Utilities|Time|SetTimerbyEvent (delegate Custom|StartFire) (Variables|Default|GetIdleTime))
  (Development|SetHiddeninGame (Variables|Default|GetFlame) true true)
  (Collision|SetCollisionEnabled (Variables|Default|GetKillZone) "NoCollision")
  (Audio|Components|Audio|Stop (stale Custom|StartFire _returnvalue)))

(event Custom|StartFire
  (Utilities|Time|SetTimerbyEvent (delegate Custom|StopFire) (Variables|Default|GetFireTime))
  (Development|SetHiddeninGame (Variables|Default|GetFlame) false true)
  (Collision|SetCollisionEnabled (Variables|Default|GetKillZone) "QueryOnly")
  (bind _returnvalue (Audio|SpawnSoundatLocation "/Game/Sounds/SFX/Fire/flamethrower2_Cue.flamethrower2_Cue" (Transformation|GetActorLocation) "0, 0, 0" 0.8)))

(event EventBeginPlay
  (Utilities|FlowControl|Delay (Variables|Default|GetBeginPlayDelay))
  (CallFunction|StartFire))

(event EventActorBeginOverlap
  (params (OtherActor :type Actor%20Object%20Reference)))

(event EventTick
  (params (DeltaSeconds :type Float%20%28single-precision%29)))

(fn ConstructionScript)
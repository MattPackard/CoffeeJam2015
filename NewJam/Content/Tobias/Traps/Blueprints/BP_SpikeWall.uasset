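; Spike wall trap that thrusts its spikes out when its trigger is overlapped and calls KillPlayer on actors the spikes touch.
; An overlap sets IsTriggered and starts a four-second timer that clears it.
; Tick eases the spikes from their current position toward the TargetPoint location while triggered, gated by TimerWasOn, which this graph never sets.
; Otherwise it eases them back to the actor's starting location.
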(event OnComponentBeginOverlap(Spikes)
  (params (OtherActor :type Actor%20Object%20Reference) (OtherComp :type Primitive%20Component%20Object%20Reference) (OtherBodyIndex :type Integer) (bFromSweep :type Boolean) (SweepResult :type Hit%20Result%20Structure%20%28by%20ref%29))
  (CallFunction|KillPlayer OtherActor))

(event OnActorBeginOverlap(Trigger)
  (params (OtherActor :type Actor%20Object%20Reference))
  (Utilities|Time|SetTimerbyEvent (delegate Custom|DisableTimer) 4.0)
  (Variables|Default|SetisTriggered true))

(event OnActorEndOverlap(Trigger)
  (params (OtherActor :type Actor%20Object%20Reference)))

(event Custom|DisableTimer
  (Variables|Default|SetisTriggered false))

(event EventBeginPlay
  (Variables|Default|SetStartLocation (Transformation|GetActorLocation))
  (Variables|Default|SetTargetLocation (Transformation|GetWorldLocation (Variables|Default|GetTargetPoint))))

(event EventTick
  (params (DeltaSeconds :type Float%20%28single-precision%29))
  (bind _spikes (Variables|Default|GetSpikes))
  (bind _spikes_2 (Variables|Default|GetSpikes))
  (bind _returnvalue (Transformation|GetWorldLocation _spikes_2))
  (if (Variables|Default|GetisTriggered)
    (if (not (Variables|Default|GettimerWasOn))
      (Transformation|SetWorldLocation _spikes (Math|Interpolation|Ease "SinusoidalIn" (Variables|Default|GetEase%20Alpha) _returnvalue (Variables|Default|GetTargetLocation)) false false))
    (else
      (Transformation|SetWorldLocation _spikes (Math|Interpolation|Ease "ExpoIn" (Variables|Default|GetEase%20Alpha) _returnvalue (Variables|Default|GetStartLocation)) false false))))

(fn ConstructionScript
  (|CallParentFunction))
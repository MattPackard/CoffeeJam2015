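; Ceiling trap that moves to a target point when triggered and kills the side-scroller character on spike contact.
; The first overlap on a Trigger actor sets IsTriggered, which nothing here resets.
; Tick then eases the trap from its start location to the TargetPoint position cached at BeginPlay, without sweeping.
; Either of two spike components calls the character's death event and adds an audio component.
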(event OnComponentBeginOverlap(Spike)
  (params (OtherActor :type Actor%20Object%20Reference) (OtherComp :type Primitive%20Component%20Object%20Reference) (OtherBodyIndex :type Integer) (bFromSweep :type Boolean) (SweepResult :type Hit%20Result%20Structure%20%28by%20ref%29))
  (bind _asside_scroller_character (Utilities|Casting|CastToSideScrollerCharacter OtherActor))
  (Default|CallOnDeath _asside_scroller_character)
  (AddComponent|AddAudioComponent false))

(event OnComponentBeginOverlap(Spike2)
  (params (OtherActor :type Actor%20Object%20Reference) (OtherComp :type Primitive%20Component%20Object%20Reference) (OtherBodyIndex :type Integer) (bFromSweep :type Boolean) (SweepResult :type Hit%20Result%20Structure%20%28by%20ref%29))
  (bind _asside_scroller_character (Utilities|Casting|CastToSideScrollerCharacter OtherActor))
  (Default|CallOnDeath _asside_scroller_character)
  (AddComponent|AddAudioComponent false))

(event OnActorBeginOverlap(Trigger)
  (params (OtherActor :type Actor%20Object%20Reference))
  (if (not (Variables|Default|GetisTriggered))
    (Variables|Default|SetisTriggered true)))

(event EventBeginPlay
  (Variables|Default|SetStartLocation (Transformation|GetActorLocation))
  (Variables|Default|SetTargetLocation (Transformation|GetWorldLocation (Variables|Default|GetTargetPoint))))

(event EventTick
  (params (DeltaSeconds :type Float%20%28single-precision%29))
  (if (Variables|Default|GetisTriggered)
    (Transformation|SetActorLocation (Math|Interpolation|VInterpTo (Transformation|GetActorLocation) (Variables|Default|GetTargetLocation) DeltaSeconds (Variables|Default|GetMoveTime)) false false)
    (else
      (Transformation|SetActorLocation (Math|Interpolation|VInterptoConstant (Transformation|GetActorLocation) (Variables|Default|GetStartLocation) DeltaSeconds (Variables|Default|GetMoveTime)) false false))))

(fn ConstructionScript
  (|CallParentFunction))
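; BP_QuickSand is a quicksand trap for the side-scroller character.
; Entering the Sand volume stores the character as Player, blocks its movement and lowers its gravity scale so it sinks slowly.
; Any end overlap on Sand, without an actor check, restores movement and sets a higher gravity scale on the stored Player.
; A separate Box volume, marking the bottom, calls CallOnDeath on the character that reaches it.
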(event OnComponentBeginOverlap(Box)
  (params (OtherActor :type Actor%20Object%20Reference) (OtherComp :type Primitive%20Component%20Object%20Reference) (OtherBodyIndex :type Integer) (bFromSweep :type Boolean) (SweepResult :type Hit%20Result%20Structure%20%28by%20ref%29))
  ;[1 0.04473 0] Handle Death When Player Reaches Bottom
  (bind _asside_scroller_character (Utilities|Casting|CastToSideScrollerCharacter OtherActor))
  (Default|CallOnDeath _asside_scroller_character))

(event OnComponentBeginOverlap(Sand)
  (params (OtherActor :type Actor%20Object%20Reference) (OtherComp :type Primitive%20Component%20Object%20Reference) (OtherBodyIndex :type Integer) (bFromSweep :type Boolean) (SweepResult :type Hit%20Result%20Structure%20%28by%20ref%29))
  (bind _asside_scroller_character (Utilities|Casting|CastToSideScrollerCharacter OtherActor))
  (Variables|Default|SetPlayer _asside_scroller_character)
  (Variables|Default|SetisTriggered true)
  (Variables|/Game/SideScrollerBP/Blueprints/SideScrollerCharacter.SideScrollerCharacter_C|SetcanPlayerMove (Variables|Default|GetPlayer) false)
  (Variables|/Script/Engine.CharacterMovementComponent|SetGravityScale (Variables|/Script/Engine.Character|GetCharacterMovement (Variables|Default|GetPlayer)) 0.1))

(event OnComponentEndOverlap(Sand)
  (params (OtherActor :type Actor%20Object%20Reference) (OtherComp :type Primitive%20Component%20Object%20Reference) (OtherBodyIndex :type Integer))
  (Variables|Default|SetisTriggered false)
  (Variables|/Game/SideScrollerBP/Blueprints/SideScrollerCharacter.SideScrollerCharacter_C|SetcanPlayerMove (Variables|Default|GetPlayer) true)
  (Variables|/Script/Engine.CharacterMovementComponent|SetGravityScale (Variables|/Script/Engine.Character|GetCharacterMovement (Variables|Default|GetPlayer)) 2.0))

(event EventBeginPlay)

(event EventTick
  (params (DeltaSeconds :type Float%20%28single-precision%29)))

(fn ConstructionScript)
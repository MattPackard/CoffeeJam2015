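; Sliding door Blueprint that moves a Cube between OpenPos and ClosedPos, starting from DefaultState.
; When a SideScrollerCharacter enters KeyTrigger, TriggerDoor opens a Gate, letting Tick interpolate toward the opposite position until within tolerance, then flip State.
; Leaving the trigger sets State false without moving the door.
; A CheckKeys function consumes RequiredKeys from a key list, but its calling branch is disconnected, so keys are never required.
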(event OnComponentBeginOverlap(KeyTrigger)
  (params (OtherActor :type Actor%20Object%20Reference) (OtherComp :type Primitive%20Component%20Object%20Reference) (OtherBodyIndex :type Integer) (bFromSweep :type Boolean) (SweepResult :type Hit%20Result%20Structure%20%28by%20ref%29))
  (bind _asside_scroller_character (Utilities|Casting|CastToSideScrollerCharacter OtherActor))
  (CallFunction|TriggerDoor))

(event OnComponentEndOverlap(KeyTrigger)
  (params (OtherActor :type Actor%20Object%20Reference) (OtherComp :type Primitive%20Component%20Object%20Reference) (OtherBodyIndex :type Integer))
  (Utilities|Casting|CastToSideScrollerCharacter OtherActor)
  (Variables|Default|SetState false))

(event Custom|Trigger%20Door
  (bind _cube (Variables|Default|GetCube))
  (bind _openpos (Variables|Default|GetOpenPos))
  (bind _closedpos (Variables|Default|GetClosedPos))
  (bind _returnvalue (Transformation|GetWorldLocation _closedpos))
  (bind _returnvalue_2 (Transformation|GetWorldLocation _openpos))
  (bind _returnvalue_3 (Transformation|GetWorldLocation _cube))
  ;[1 1 1] Animation Event
  (Utilities|FlowControl|Gate true) ; enters at Open
)

(event EventBeginPlay
  ;[1 1 1] Initialisation
  (bind _output_get (Variables|Default|SetState (Variables|Default|GetDefault%20State)))
  (if _output_get
    (Transformation|SetWorldLocation (Variables|Default|GetCube) (Transformation|GetWorldLocation (Variables|Default|GetOpenPos)) false false)
    (else
      (Transformation|SetWorldLocation (Variables|Default|GetCube) (Transformation|GetWorldLocation (Variables|Default|GetClosedPos)) false false))))

(event EventTick
  (params (DeltaSeconds :type Float%20%28single-precision%29))
  (bind _cube (Variables|Default|GetCube))
  (bind _openpos (Variables|Default|GetOpenPos))
  (bind _closedpos (Variables|Default|GetClosedPos))
  (bind _returnvalue (Transformation|GetWorldLocation _closedpos))
  (bind _returnvalue_2 (Transformation|GetWorldLocation _openpos))
  (bind _returnvalue_3 (Transformation|GetWorldLocation _cube))
  ;[1 1 1] Animation Event
  (Utilities|FlowControl|Gate true :!label _label
    (:Exit
      (if (Variables|Default|GetState)
        (CallFunction|Interp _returnvalue_3 _returnvalue _cube DeltaSeconds)
        (if (Math|Vector|Equal(Vector) _returnvalue _returnvalue_3 1e+01)
          (Variables|Default|SetState false)
          (goto _label Close))
        (else
          (CallFunction|Interp _returnvalue_3 _returnvalue_2 _cube DeltaSeconds)
          (if (Math|Vector|Equal(Vector) _returnvalue_3 _returnvalue_2 1e+01)
            (Variables|Default|SetState true)
            (goto _label Close)))))))

(fn ConstructionScript)

(fn Interp
  (params (Start :type Vector) (End :type Vector) (Mesh :type Static%20Mesh%20Component%20Object%20Reference) (Delta :type Float%20%28single-precision%29))
  (Transformation|SetWorldLocation Mesh (Math|Interpolation|VInterpTo Start End Delta (Variables|Default|GetOpen%20Speed)) false false))

(fn CheckKeys
  (params (Keys :type Array%20of%20Integers))
  (bind _array_element (Utilities|Array|ForEachLoopwithBreak (Variables|Default|GetRequiredKeys))
    (:LoopBody
      (if (> (Utilities|Array|FindItem Keys _array_element) -1)
        (Utilities|Array|RemoveIndex Keys (Utilities|Array|FindItem Keys _array_element))
        (else
          (return false))))
    (:Completed
      (return true))))
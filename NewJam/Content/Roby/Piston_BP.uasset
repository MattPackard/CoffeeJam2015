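; Piston actor that extends along world X by a set distance when triggered, then retracts to its starting position.
; TriggerPiston records the current location as the start, computes the end point and opens a gate on Tick.
; While the gate is open, the actor eases toward the target with VInterpTo, flips to retract on arrival, and closes the gate once back home.
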(event Custom|Trigger%20Piston
  (bind _output_get (Variables|Default|SetInitialPos (Transformation|GetWorldLocation (Variables|Default|GetPiston))))
  (Variables|Default|SetRetract false)
  (Variables|Default|SetFinalPos (Math|Vector|MakeVector (+ (Variables|Default|GetDistance) (.X (Math|Vector|BreakVector _output_get))) (.Y (Math|Vector|BreakVector _output_get)) (.Z (Math|Vector|BreakVector _output_get))))
  (Utilities|FlowControl|Gate true) ; enters at Open
)

(event EventTick
  (params (DeltaSeconds :type Float%20%28single-precision%29))
  (Utilities|FlowControl|Gate true :!label _label
    (:Exit
      (if (Variables|Default|GetRetract)
        (Transformation|SetActorLocation (Math|Interpolation|VInterpTo (Transformation|GetWorldLocation (Variables|Default|GetPiston)) (Variables|Default|GetInitialPos) DeltaSeconds (Variables|Default|GetSpeed)) false false)
        (if (Math|Vector|Equal(Vector) (Variables|Default|GetInitialPos) (Transformation|GetWorldLocation (Variables|Default|GetPiston)) 1.0)
          (goto _label Close))
        (else
          (Transformation|SetActorLocation (Math|Interpolation|VInterpTo (Transformation|GetWorldLocation (Variables|Default|GetPiston)) (Variables|Default|GetFinalPos) DeltaSeconds (Variables|Default|GetSpeed)) false false)
          (if (Math|Vector|Equal(Vector) (Variables|Default|GetFinalPos) (Transformation|GetWorldLocation (Variables|Default|GetPiston)) 1.0)
            (Variables|Default|SetRetract true)))))))

(fn ConstructionScript)